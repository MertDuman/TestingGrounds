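; AIController_BP is an AI controller for a guard enemy that senses and tracks targets.
; On BeginPlay it sets up the PatrolData blackboard and runs the GuardBehavior behavior tree.
; Perception updates write the sensed actor into the blackboard enemy key, and clear that key when the stimulus is lost, leaving the reaction to the behavior tree.
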(event `self.ReceiveBeginPlay`
  (bind _blackboardcomponent (`self.UseBlackboard` "/Game/Dynamic/AI/Behavior/PatrolData.PatrolData"))
  (`self.RunBehaviorTree` "/Game/Dynamic/AI/Behavior/GuardBehavior.GuardBehavior")
  (set `self.BlackboardComp` _blackboardcomponent))

(event `self.AIPerception.OnTargetPerceptionUpdated`
  (params (Actor :type "Actor Object Reference") (Stimulus :type "AIStimulus Structure"))
  (if (`.bSuccessfullySensed` (break `AIStimulus` Stimulus))
    (`BlackboardComponent.SetValueAsObject` (`self.Blackboard`) (`self.BlackboardEnemyKeyName`) Actor)
    (else
      (`BlackboardComponent.ClearValue` (`self.Blackboard`) (`self.BlackboardEnemyKeyName`)))))

(fn `UserConstructionScript`)